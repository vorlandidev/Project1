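; Blueprint math function library with a helper that turns 2D input into a horizontal world-space direction relative to a given scene component.
; It flattens the component's forward and right vectors to the XY plane and normalizes them.
; Input Y scales forward and X scales right, and their sum is optionally normalized.
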(fn `InputToWorldDirection`
  (params (`Scene Component` :type "SceneComponent Object Reference") (`Vector 2D` :type "Vector2D Structure") (`Normalize Output` :type Boolean))
  (returns (`Movement Direction` :type "Vector Structure"))
  (bind (_x _y) (`KismetMathLibrary.BreakVector2D` `Vector 2D`))
  (bind _returnvalue (+ (* _y (`KismetMathLibrary.Normal` (`KismetMathLibrary.MakeVector` (.x (`SceneComponent.GetForwardVector` `Scene Component`)) (.y (`SceneComponent.GetForwardVector` `Scene Component`))))) (* _x (`KismetMathLibrary.Normal` (`KismetMathLibrary.MakeVector` (.x (`SceneComponent.GetRightVector` `Scene Component`)) (.y (`SceneComponent.GetRightVector` `Scene Component`)))))))
  (return (select `bool` `Normalize Output` :`false` _returnvalue :`true` (`KismetMathLibrary.Normal` _returnvalue))))