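; Player actor component for a camera that leads movement and a character that turns to face the mouse cursor.
; Each tick it smoothly shifts the owner's spring arm target offset along the arm's yaw-relative move input, scaled by a lead distance.
; It also intersects the deprojected cursor ray with a horizontal plane at the owner's height and interpolates the actor's rotation toward that point.
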(event `self.ReceiveBeginPlay`
  (set `self.SpringArmReference` (`Actor.GetComponentByClass` (`self.GetOwner`) "/Script/Engine.SpringArmComponent"))
  (set `self.CameraReference` (`Actor.GetComponentByClass` (`self.GetOwner`) "/Script/Engine.CameraComponent")))

(event `self.ReceiveTick`
  (params (DeltaSeconds :type "Float (single-precision)"))
  (bind (_x _y) (`KismetMathLibrary.BreakVector2D` (`self.MoveInput`)))
  (bind _returnvalue (`KismetMathLibrary.MakeRotator` 0.0 0.0 (.yaw (`SpringArmComponent.GetTargetRotation` (`self.SpringArmReference`)))))
  (bind _output_get (set `self.CurrentCameraOffset` (`KismetMathLibrary.VInterpTo` (`self.CurrentCameraOffset`) (* (+ (* (`KismetMathLibrary.GetRightVector` _returnvalue) _x) (* (`KismetMathLibrary.GetForwardVector` _returnvalue) _y)) (`self.CameraLeadDistance`)) DeltaSeconds 3.0)))
  (set `SpringArmComponent.TargetOffset` _output_get (`self.SpringArmReference`))
  (`self.UpdateMouseRotation` DeltaSeconds))

(fn `SetMoveInput`
  (params (NewMoveInput :type "Vector2D Structure"))
  (set `self.MoveInput` NewMoveInput))

(fn `UpdateMouseRotation`
  (params (DeltaTime :type "Float (double-precision)"))
  (bind (_worldlocation _worlddirection) (`PlayerController.DeprojectMousePositionToWorld` (`GameplayStatics.GetPlayerController` 0)))
  (bind _returnvalue (`Actor.K2_GetActorLocation` (`self.GetOwner`)))
  (bind (_t _intersection _returnvalue_2) (`KismetMathLibrary.LinePlaneIntersection` _worldlocation (+ _worldlocation (* _worlddirection (`self.WorldLineMultiplier`))) (`KismetMathLibrary.MakePlaneFromPointAndNormal` _returnvalue (0.0 0.0 1.0))))
  (if _returnvalue_2
    (`Actor.K2_SetActorRotation` (`self.GetOwner`) (`KismetMathLibrary.RInterpTo` (`Actor.K2_GetActorRotation` (`self.GetOwner`)) (`KismetMathLibrary.FindLookAtRotation` _returnvalue _intersection) DeltaTime 8.0) false)))