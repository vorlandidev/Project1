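; Player character Blueprint that handles camera-relative movement and a dash with a cooldown.
; Move input drives movement along the spring arm's yaw, is passed to the camera follow component and is cleared on release.
; Dash turns the stored input into a world direction, then a timeline lerps the actor a set distance with a swept location update.
; Normal movement pauses during the dash, and a timer re-enables dashing afterwards.
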(event `EnhancedInput|/Game/Input/Actions/IA_Dash`
  (params (ActionValue :type Boolean) (ElapsedSeconds :type "Float (double-precision)") (TriggeredSeconds :type "Float (double-precision)") (InputAction :type "InputAction Object Reference" :default "/Game/Input/Actions/IA_Dash.IA_Dash"))
  (:`Started`
    (if (`self.CanDash`)
      (set `self.CanDash` false)
      (set `self.IsDashing` true)
      (bind _output_get (set `self.DashStartLocation` (`self.K2_GetActorLocation`)))
      (bind _output_get_2 (set `self.DashDirection` (`/Game/Blueprints/BPFL_Math/BPFL_Math.InputToWorldDirection` (`self.SpringArm`) (`self.MoveInput`) true)))
      (bind _output_get_3 (set `self.DashEndLocation` (+ (* (`self.DashDistance`) _output_get_2) _output_get)))
      (bind (_direction _dashalpha) (`Timeline|TL_Dash` :!via `PlayFromStart`)
        (:`Update`
          (`self.K2_SetActorLocation` (`KismetMathLibrary.VLerp` _output_get _output_get_3 _dashalpha) true))
        (:`Finished`
          (set `self.IsDashing` false)
          (`KismetSystemLibrary.K2_SetTimerDelegate` (delegate `ResetDash`) (`self.DashCooldown`)))))))

(event `ResetDash`
  (set `self.CanDash` true))

(event `EnhancedInput|/Game/Input/Actions/IA_Move`
  (params (ActionValue :type "Vector2D Structure") (ElapsedSeconds :type "Float (double-precision)") (TriggeredSeconds :type "Float (double-precision)") (InputAction :type "InputAction Object Reference" :default "/Game/Input/Actions/IA_Move.IA_Move"))
  (bind (_x _y) (`KismetMathLibrary.BreakVector2D` ActionValue))
  (bind _returnvalue (`KismetMathLibrary.MakeRotator` 0.0 0.0 (.yaw (`SpringArmComponent.GetTargetRotation` (`self.SpringArm`)))))
  (:`Triggered`
    (bind _output_get (set `self.MoveInput` ActionValue))
    (if (not (`self.IsDashing`))
      (`self.AddMovementInput` (`KismetMathLibrary.GetRightVector` _returnvalue) _x)
      (`self.AddMovementInput` (`KismetMathLibrary.GetForwardVector` _returnvalue) _y)
      (`/Game/Blueprints/BP_CameraFollowComponent.SetMoveInput` (`self.BP_CameraFollowComponent`) _output_get)))
  (:`Canceled`
    (bind _output_get_2 (set `self.MoveInput` (0.0 0.0) :!label _label))
    (`/Game/Blueprints/BP_CameraFollowComponent.SetMoveInput` (`self.BP_CameraFollowComponent`) _output_get_2))
  (:`Completed`
    (goto _label)))

(fn `UserConstructionScript`)