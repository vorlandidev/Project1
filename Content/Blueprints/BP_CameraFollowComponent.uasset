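; BP_CameraFollowComponent is a component that leads its owner's camera in the direction of movement input.
; BeginPlay caches the owner's spring arm and camera, and SetMoveInput stores the input supplied by callers.
; Each tick maps that input onto the spring arm's yaw-only right and forward axes, scales it by CameraLeadDistance, and smoothly interpolates the arm's TargetOffset toward it.
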(event `self.ReceiveBeginPlay`
  (set `self.SpringArmReference` (`Actor.GetComponentByClass` (`self.GetOwner`) "/Script/Engine.SpringArmComponent"))
  (set `self.CameraReference` (`Actor.GetComponentByClass` (`self.GetOwner`) "/Script/Engine.CameraComponent")))

(event `self.ReceiveTick`
  (params (DeltaSeconds :type "Float (single-precision)"))
  (bind (_x _y) (`KismetMathLibrary.BreakVector2D` (`self.MoveInput`)))
  (bind _returnvalue (`KismetMathLibrary.MakeRotator` 0.0 0.0 (.yaw (`SpringArmComponent.GetTargetRotation` (`self.SpringArmReference`)))))
  (bind _output_get (set `self.CurrentCameraOffset` (`KismetMathLibrary.VInterpTo` (`self.CurrentCameraOffset`) (* (+ (* (`KismetMathLibrary.GetRightVector` _returnvalue) _x) (* (`KismetMathLibrary.GetForwardVector` _returnvalue) _y)) (`self.CameraLeadDistance`)) DeltaSeconds 3.0)))
  (set `SpringArmComponent.TargetOffset` _output_get (`self.SpringArmReference`)))

(fn `SetMoveInput`
  (params (NewMoveInput :type "Vector2D Structure"))
  (set `self.MoveInput` NewMoveInput))